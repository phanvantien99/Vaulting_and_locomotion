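; BP_Dummy is a damageable dummy character that reacts to hits with animation and is destroyed once its health runs out.
; On AnyDamage it subtracts the damage from MaxHealth, which doubles as current health, and plays one of three random damage montages.
; Health is checked before subtraction, so the actor is destroyed on the next damage event after health reaches zero or below.
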(event `self.ReceiveAnyDamage`
  (params (Damage :type "Float (single-precision)") (DamageType :type "DamageType Object Reference") (InstigatedBy :type "Controller Object Reference") (DamageCauser :type "Actor Object Reference"))
  (if (> (`self.MaxHealth`) 0.0)
    (set `self.MaxHealth` (- (`self.MaxHealth`) Damage))
    (bind _output_get (set `self.RandomPose` (`KismetMathLibrary.RandomIntegerInRange` 0 2)))
    (switch `int` _output_get
      (:`0`
        (`self.PlayAnimMontage` "/Game/Characters/Mannequins/Animations/Manny/Montages/Damaged1.Damaged1"))
      (:`1`
        (`self.PlayAnimMontage` "/Game/Characters/Mannequins/Animations/Manny/Montages/Damaged2.Damaged2"))
      (:`2`
        (`self.PlayAnimMontage` "/Game/Characters/Mannequins/Animations/Manny/Montages/damaged3.damaged3")))
    (else
      (`self.K2_DestroyActor`))))

(fn `UserConstructionScript`)