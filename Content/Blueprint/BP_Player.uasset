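; Player character with Enhanced Input movement, look, jump, timeline-zoomed sprint and vaulting over obstacles.
; The vault input runs VaultNext, which traces forward, then downward along the obstacle to find start, middle and landing points.
; The warp event disables collision, switches to Flying and plays the vault montage, writing all three points to one "StartWarp" Motion Warping target.
; An older Vault trace routine remains, called only from unconnected nodes.
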(event `self.ReceivePossessed`
  (params (NewController :type "Controller Object Reference"))
  ;[0.3781 1 0.8077 1 30] Configure the input
  (bind _asplayer_controller (cast `PlayerController` NewController))
  (`EnhancedInputSubsystemInterface.AddMappingContext` (pcsubsystem `EnhancedInputLocalPlayerSubsystem` _asplayer_controller) "/Game/Blueprint/Inputs/IM_Control.IM_Control" 0 (struct)))

(event `EnhancedInput|/Game/Blueprint/Inputs/IA_Forward`
  (params (ActionValue :type "Float (double-precision)") (ElapsedSeconds :type "Float (double-precision)") (TriggeredSeconds :type "Float (double-precision)") (InputAction :type "InputAction Object Reference" :default "/Game/Blueprint/Inputs/IA_Forward.IA_Forward"))
  (bind (_returnvalue_roll _returnvalue_pitch _returnvalue_yaw) (`KismetMathLibrary.BreakRotator` (`self.GetControlRotation`)))
  ;[1 1 1] Configure movement
  (:`Triggered`
    (if (not (`self.isAttacking`))
      (`self.AddMovementInput` (`KismetMathLibrary.GetForwardVector` (`KismetMathLibrary.MakeRotator` 0.0 0.0 _returnvalue_yaw)) ActionValue))))

(event `EnhancedInput|/Game/Blueprint/Inputs/IA_Turn`
  (params (ActionValue :type "Float (double-precision)") (ElapsedSeconds :type "Float (double-precision)") (TriggeredSeconds :type "Float (double-precision)") (InputAction :type "InputAction Object Reference" :default "/Game/Blueprint/Inputs/IA_Turn.IA_Turn"))
  ;[0.3094 0.3094 0.3094] Configure for mouse rotation
  (:`Triggered`
    (`self.AddControllerYawInput` ActionValue)))

(event `EnhancedInput|/Game/Blueprint/Inputs/IA_LookUp`
  (params (ActionValue :type "Float (double-precision)") (ElapsedSeconds :type "Float (double-precision)") (TriggeredSeconds :type "Float (double-precision)") (InputAction :type "InputAction Object Reference" :default "/Game/Blueprint/Inputs/IA_LookUp.IA_LookUp"))
  ;[0.3094 0.3094 0.3094] Configure for mouse rotation
  (:`Triggered`
    (`self.AddControllerPitchInput` ActionValue)))

(event `EnhancedInput|/Game/Blueprint/Inputs/IA_MoveRight`
  (params (ActionValue :type "Float (double-precision)") (ElapsedSeconds :type "Float (double-precision)") (TriggeredSeconds :type "Float (double-precision)") (InputAction :type "InputAction Object Reference" :default "/Game/Blueprint/Inputs/IA_MoveRight.IA_MoveRight"))
  (bind (_returnvalue_roll _returnvalue_pitch _returnvalue_yaw) (`KismetMathLibrary.BreakRotator` (`self.GetControlRotation`)))
  ;[1 1 1] Configure movement
  (:`Triggered`
    (if (not (`self.isAttacking`))
      (`self.AddMovementInput` (`KismetMathLibrary.GetRightVector` (`KismetMathLibrary.MakeRotator` _returnvalue_roll 0.0 _returnvalue_yaw)) ActionValue))))

(event `EnhancedInput|/Game/Blueprint/Inputs/IA_Jump`
  (params (ActionValue :type Boolean) (ElapsedSeconds :type "Float (double-precision)") (TriggeredSeconds :type "Float (double-precision)") (InputAction :type "InputAction Object Reference" :default "/Game/Blueprint/Inputs/IA_Jump.IA_Jump"))
  ;[1 1 1] Jumping
  (:`Triggered`
    (switch `EMovementMode` (`CharacterMovementComponent.MovementMode` (`self.CharacterMovement`))
      (:`MOVE_Walking`
        (`self.Jump`))))
  (:`Completed`
    (`self.StopJumping`)))

(event `EnhancedInput|/Game/Blueprint/Inputs/IA_Sprint`
  (params (ActionValue :type Boolean) (ElapsedSeconds :type "Float (double-precision)") (TriggeredSeconds :type "Float (double-precision)") (InputAction :type "InputAction Object Reference" :default "/Game/Blueprint/Inputs/IA_Sprint.IA_Sprint"))
  ;[1 1 1] Spinting
  (:`Triggered`
    (switch `EMovementMode` (`CharacterMovementComponent.MovementMode` (`self.CharacterMovement`))
      (:`MOVE_Walking`
        (set `CharacterMovementComponent.MaxWalkSpeed` 700.0 (`self.CharacterMovement`))
        (bind (_direction _cam_length) (`Timeline|Camera Zoom` :!label _label)
          (:`Update`
            (set `SpringArmComponent.TargetArmLength` (`KismetMathLibrary.Lerp` 500.0 300.0 _cam_length) (`self.Follow SpringArm`)))))))
  (:`Completed`
    (set `CharacterMovementComponent.MaxWalkSpeed` 450.0 (`self.CharacterMovement`))
    (`KismetSystemLibrary.Delay` 3.0)
    (goto _label :!via `Reverse`)))

(event `EnhancedInput|/Game/Blueprint/Inputs/IA_Vault`
  (params (ActionValue :type Boolean) (ElapsedSeconds :type "Float (double-precision)") (TriggeredSeconds :type "Float (double-precision)") (InputAction :type "InputAction Object Reference" :default "/Game/Blueprint/Inputs/IA_Vault.IA_Vault"))
  (:`Triggered`
    (`self.Vault Next`)))

(event `WarpMotionEent`
  (bind (_vaultlandpos_x _vaultlandpos_y _vaultlandpos_z) (`KismetMathLibrary.BreakVector` (`self.VaultLandPos`)))
  (bind (_returnvalue_x _returnvalue_y _returnvalue_z) (`KismetMathLibrary.BreakVector` (`SceneComponent.K2_GetComponentLocation` (`self.Mesh`))))
  ;[1 1 1] Event Warp motion
  (if (and (`self.CanWarp`) (`KismetMathLibrary.InRange_FloatFloat` _vaultlandpos_z (- _returnvalue_z 50.0) (+ _returnvalue_z 50.0)))
    (`CharacterMovementComponent.SetMovementMode` (`self.CharacterMovement`) "MOVE_Flying" 0)
    (`self.SetActorEnableCollision` false)
    (`|PlayMontage` (`self.Mesh`) "/Game/Characters/Mannequins/Animations/Quinn/Montage/MT_VaultOver.MT_VaultOver"
      (:`OnCompleted`
        (`CharacterMovementComponent.SetMovementMode` (`self.CharacterMovement`) "MOVE_Walking" 0)
        (`self.SetActorEnableCollision` true)
        (set `self.CanWarp` false)
        (set `self.VaultLandPos` (0.0 0.0 20000.0))))))

(event `Warp_motion_CC`
  (`|ExecutionSequence`
    (:`then_0`
      (`KismetSystemLibrary.DrawDebugSphere` (`self.VaultStart`) 5.0 12 (struct :`G` 1.0 :`B` 0.081708 :`A` 1.0) 60.0)
      (`KismetSystemLibrary.DrawDebugSphere` (`self.VaultMiddle`) 5.0 12 (struct :`R` 1.0 :`G` 0.815095 :`A` 1.0) 60.0)
      (`KismetSystemLibrary.DrawDebugSphere` (`self.VaultLand`) 5.0 12 (struct :`R` 1.0 :`G` 0.036887 :`A` 1.0) 60.0))
    (:`then_1`
      (`CharacterMovementComponent.SetMovementMode` (`self.CharacterMovement`) "MOVE_Flying" 0)
      (`self.SetActorEnableCollision` false)
      (`MotionWarpingComponent.AddOrUpdateWarpTarget` (`self.MotionWarping`) "StartWarp" (make `MotionWarpingTarget` (`KismetMathLibrary.MakeTransform` (`self.VaultStart`) (`self.K2_GetActorRotation`))))
      (`MotionWarpingComponent.AddOrUpdateWarpTarget` (`self.MotionWarping`) "StartWarp" (make `MotionWarpingTarget` (`KismetMathLibrary.MakeTransform` (`self.VaultMiddle`) (`self.K2_GetActorRotation`))))
      (`MotionWarpingComponent.AddOrUpdateWarpTarget` (`self.MotionWarping`) "StartWarp" (make `MotionWarpingTarget` (`KismetMathLibrary.MakeTransform` (`self.VaultLand`) (`self.K2_GetActorRotation`))))
      (`|PlayMontage` (`self.Mesh`) "/Game/Characters/Mannequins/Animations/Quinn/Montage/MT_VaultOver.MT_VaultOver"
        (:`OnCompleted`
          (`CharacterMovementComponent.SetMovementMode` (`self.CharacterMovement`) "MOVE_Walking" 0)
          (`self.SetActorEnableCollision` true)
          (set `self.CanWarp_CC` false))))))

(fn `UserConstructionScript`
  (set `self.WalkSpeed` (`CharacterMovementComponent.MaxWalkSpeed` (`self.CharacterMovement`))))

(fn `Vault`
  (for _index (range 3)
    (bind _returnvalue (+ (`self.K2_GetActorLocation`) (`KismetMathLibrary.MakeVector` 0.0 0.0 (* _index 30))))
    (bind (_outhit _returnvalue_2) (`KismetSystemLibrary.SphereTraceSingle` :`Start` _returnvalue :`End` (+ _returnvalue (* (`KismetMathLibrary.GetForwardVector` (`self.K2_GetActorRotation`)) 300.0)) :`Radius` 5.0 :`TraceChannel` "TraceTypeQuery1" :`DrawDebugType` "ForDuration"))
    (if _returnvalue_2
      (`|ExecutionSequence`
        (:`then_0`
          (break))
        (:`then_1`
          (for _index_2 (range 6)
            (bind _returnvalue_3 (+ (* (* _index_2 50) (`KismetMathLibrary.GetForwardVector` (`self.K2_GetActorRotation`))) (+ (`.Location` (`GameplayStatics.BreakHitResult` _outhit)) (0.0 0.0 100.0))))
            (bind (_outhit_2 _returnvalue_4) (`KismetSystemLibrary.SphereTraceSingle` :`Start` _returnvalue_3 :`End` (- _returnvalue_3 (0.0 0.0 100.0)) :`Radius` 10.0 :`TraceChannel` "TraceTypeQuery1" :`DrawDebugType` "ForDuration"))
            (if _returnvalue_4
              (`|ExecutionSequence`
                (:`then_0`
                  (if (== _index_2 0)
                    (bind (_bblockinghit _binitialoverlap _time _distance _location _impactpoint _normal _impactnormal _physmat _hitactor _hitcomponent _hitbonename _bonename _hititem _elementindex _faceindex _tracestart _traceend) (`GameplayStatics.BreakHitResult` _outhit_2))
                    (bind _output_get (set `self.VaultStartPos` _location))
                    (`KismetSystemLibrary.DrawDebugSphere` _output_get 10.0 12 (struct :`G` 0.070262 :`B` 1.0 :`A` 1.0) 10.0)))
                (:`then_1`
                  (bind _output_get_2 (set `self.VaultMiddlePos` _location))
                  (`KismetSystemLibrary.DrawDebugSphere` _output_get_2 10.0 12 (struct :`R` 0.986268 :`B` 1.0 :`A` 1.0) 10.0)
                  (set `self.CanWarp` true)))
              (else
                (bind _returnvalue_5 (+ _traceend (* (`KismetMathLibrary.GetForwardVector` (`self.K2_GetActorRotation`)) 80.0)))
                (bind (_outhit_3 _returnvalue_6) (`KismetSystemLibrary.LineTraceSingle` :`Start` _returnvalue_5 :`End` (- _returnvalue_5 (0.0 0.0 1000.0)) :`TraceChannel` "TraceTypeQuery1" :`TraceColor` (struct :`G` 0.961045 :`B` 1.0 :`A` 1.0) :`TraceHitColor` (struct :`R` 0.984897 :`G` 1.0 :`A` 1.0)))
                (if _returnvalue_6
                  (set `self.VaultLandPos` (`.Location` (`GameplayStatics.BreakHitResult` _outhit_3)))
                  (break)))))
          (`self.WarpMotionEent`))))))

(fn `Vault Next`
  (bind _returnvalue (+ (`self.K2_GetActorLocation`) (0.0 0.0 30.0)))
  (bind (_outhit _returnvalue_2) (`KismetSystemLibrary.SphereTraceSingle` _returnvalue (+ _returnvalue (* (`KismetMathLibrary.GetForwardVector` (`self.K2_GetActorRotation`)) 65.0)) 5.0 "TraceTypeQuery1"))
  (if _returnvalue_2
    (for _index (range 1 6)
      (bind _returnvalue_3 (+ (* (* _index 30) (`KismetMathLibrary.GetForwardVector` (`self.K2_GetActorRotation`))) (+ (`.Location` (`GameplayStatics.BreakHitResult` _outhit)) (0.0 0.0 100.0))))
      (bind (_outhit_2 _returnvalue_4) (`KismetSystemLibrary.SphereTraceSingle` :`Start` _returnvalue_3 :`End` (- _returnvalue_3 (0.0 0.0 100.0)) :`Radius` 5.0 :`TraceChannel` "TraceTypeQuery1" :`TraceColor` (struct :`G` 0.171807 :`B` 1.0 :`A` 1.0) :`TraceHitColor` (struct :`R` 1.0 :`G` 0.971536 :`A` 1.0)))
      (if _returnvalue_4
        (if (== _index 1)
          (bind (_bblockinghit _binitialoverlap _time _distance _location _impactpoint _normal _impactnormal _physmat _hitactor _hitcomponent _hitbonename _bonename _hititem _elementindex _faceindex _tracestart _traceend) (`GameplayStatics.BreakHitResult` _outhit_2))
          (set `self.VaultStart` _location)
          (else
            (set `self.VaultMiddle` _location)))
        (else
          (bind (_outhit_3 _returnvalue_5) (`KismetSystemLibrary.LineTraceSingle` :`Start` (+ _traceend (0.0 0.0 100.0)) :`End` (- _traceend (0.0 0.0 1000.0)) :`TraceChannel` "TraceTypeQuery1" :`TraceColor` (struct :`R` 1.0 :`G` 0.66858 :`A` 1.0) :`TraceHitColor` (struct :`G` 0.948121 :`B` 1.0 :`A` 1.0)))
          (if _returnvalue_5
            (set `self.VaultLand` (+ (`.Location` (`GameplayStatics.BreakHitResult` _outhit_3)) (* (`KismetMathLibrary.GetForwardVector` (`self.K2_GetActorRotation`)) 20.0)))
            (set `self.CanWarp_CC` true)
            (break)))))
    (`self.Warp_motion_CC`)))